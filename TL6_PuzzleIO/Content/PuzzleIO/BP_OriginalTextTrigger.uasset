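; Puzzle trigger actor that gives success or failure feedback through the level's floating text.
; On BeginPlay it caches every TextRenderActor in the level and, with authority, turns on replication and movement replication for itself.
; Any actor overlap sets all cached texts to a green success message, and any overlap end sets them to a red failure message.
; Text changes use no RPCs or replicated variables.
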(event EventBeginPlay
  (bind _outactors (Actor|GetAllActorsOfClass "/Script/Engine.TextRenderActor"))
  (Variables|Default|SetAllFlavourText _outactors)
  (if (Ability|HasAuthority)
    (Networking|SetReplicates true)
    (Class|Actor|SetReplicateMovement true)))

(event Collision|EventActorBeginOverlap
  (params (OtherActor :type Actor%20Object%20Reference))
  (for _array_element (Variables|Default|GetAllFlavourText)
    (bind _astext_render_actor (Utilities|Casting|CastToTextRenderActor _array_element))
    (Rendering|Components|TextRender|SetText (Variables|/Script/Engine.TextRenderActor|GetTextRender _astext_render_actor) (Utilities|Text|ToText(String) "You did it!"))
    (Rendering|Components|TextRender|SetTextRenderColor (Variables|/Script/Engine.TextRenderActor|GetTextRender _astext_render_actor) (Math|Color|MakeColor 0 255 100))))

(event Collision|EventActorEndOverlap
  (params (OtherActor :type Actor%20Object%20Reference))
  (for _array_element (Variables|Default|GetAllFlavourText)
    (bind _astext_render_actor (Utilities|Casting|CastToTextRenderActor _array_element))
    (Rendering|Components|TextRender|SetText (Variables|/Script/Engine.TextRenderActor|GetTextRender _astext_render_actor) (Utilities|Text|ToText(String) "Whoops! Err..."))
    (Rendering|Components|TextRender|SetTextRenderColor (Variables|/Script/Engine.TextRenderActor|GetTextRender _astext_render_actor) (Math|Color|MakeColor 0 25 255))))

(fn ConstructionScript)